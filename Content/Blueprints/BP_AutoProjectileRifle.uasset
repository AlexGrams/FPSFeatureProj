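; BP_AutoProjectileRifle is a rifle pickup that attaches its TPWeapon component to the character that picks it up.
; On BeginPlay it copies its ammo, damage, fire interval, automatic and hitscan variables into TPWeapon, starting at full ammo.
; It async loads the fire animation, projectile class and fire sound, starting each without waiting on the previous, and assigns each to TPWeapon on completion.
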(event OnPickUp(TP_PickUp)
  (params (PickUpCharacter :type FPS%20Feature%20Proj%20Character%20Object%20Reference))
  (bind _tp_weapon (Variables|Default|GetTP_Weapon))
  (if (Utilities|IsValid _tp_weapon)
    (Class|TPWeaponComponent|AttachWeapon _tp_weapon PickUpCharacter)))

(event EventBeginPlay
  (bind _tp_weapon (Variables|Default|GetTP_Weapon))
  ;[1 1 1] Set instance variable on BeginPlay
  (bind _output_get (Variables|/Script/FPSFeatureProj.TP_WeaponComponent|SetMaxAmmo _tp_weapon (Variables|Default|GetMaxAmmo)))
  (Variables|/Script/FPSFeatureProj.TP_WeaponComponent|SetCurrentAmmo _tp_weapon _output_get)
  (Variables|/Script/FPSFeatureProj.TP_WeaponComponent|SetDamage _tp_weapon (Variables|Default|GetDamage))
  (Variables|/Script/FPSFeatureProj.TP_WeaponComponent|SetFireInterval _tp_weapon (Variables|Default|GetFireInterval))
  (Variables|/Script/FPSFeatureProj.BaseWeaponComponent|SetbIsAutomatic _tp_weapon (Variables|Default|GetIsAutomatic))
  (Variables|/Script/FPSFeatureProj.TP_WeaponComponent|SetIsHitscan _tp_weapon (Variables|Default|GetIsHitscan))
  (bind _object (Utilities|AsyncLoadAsset (Variables|Default|GetFireAnimation))
    (:then
      (bind _class (Utilities|AsyncLoadClassAsset (Variables|Default|GetProjectileClass))
        (:then
          (bind _object_2 (Utilities|AsyncLoadAsset (Variables|Default|GetFireSound))
            (:Completed
              (bind _assound_base (Utilities|Casting|CastToSoundBase _object_2))
              (Variables|/Script/FPSFeatureProj.TP_WeaponComponent|SetFireSound _tp_weapon _assound_base))))
        (:Completed
          (bind _asfpsfeature_proj_projectile (Utilities|Casting|CastToFPSFeatureProjProjectileClass _class))
          (Variables|/Script/FPSFeatureProj.TP_WeaponComponent|SetProjectileClass _tp_weapon _asfpsfeature_proj_projectile))))
    (:Completed
      (bind _asanim_montage (Utilities|Casting|CastToAnimMontage _object))
      (Variables|/Script/FPSFeatureProj.TP_WeaponComponent|SetFireAnimation _tp_weapon _asanim_montage))))

(fn ConstructionScript)