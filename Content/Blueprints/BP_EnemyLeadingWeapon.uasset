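; Enemy weapon actor that wraps an EnemyWeaponLeading component and can itself be damaged and destroyed.
; The construction script copies ammo, fire interval and damage settings into that component, starts it at full ammo and makes it automatic.
; Damage taken is also applied to the parent actor that owns the weapon, keeping the instigator, causer and damage type.
; When its health is depleted, the weapon destroys itself.
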(event EventHealthDepleted
  (Actor|DestroyActor))

(event EventDamageTaken
  (params (DamagedActor :type Actor%20Object%20Reference) (Damage :type Float%20%28single-precision%29) (DamageType :type Damage%20Type%20Object%20Reference) (InstigatedBy :type Controller%20Object%20Reference) (DamageCauser :type Actor%20Object%20Reference))
  ;[1 1 1] Also damage the owner of this Weapon
  (Game|Damage|ApplyDamage (Actor|GetParentActor self) Damage InstigatedBy DamageCauser (Utilities|GetClass DamageType)))

(fn ConstructionScript
  (bind _enemyweaponleading (Variables|Default|GetEnemyWeaponLeading))
  (bind _output_get (Variables|/Script/FPSFeatureProj.BaseWeaponComponent|SetMaxAmmo _enemyweaponleading (Variables|Default|GetMax%20Ammo)))
  (Variables|/Script/FPSFeatureProj.BaseWeaponComponent|SetCurrentAmmo _enemyweaponleading _output_get)
  (Variables|/Script/FPSFeatureProj.BaseWeaponComponent|SetFireInterval _enemyweaponleading (Variables|Default|GetFire%20Interval))
  (Variables|/Script/FPSFeatureProj.BaseWeaponComponent|SetDamage _enemyweaponleading (Variables|Default|GetDamage))
  (Variables|/Script/FPSFeatureProj.BaseWeaponComponent|SetbIsAutomatic _enemyweaponleading true))