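; BP_Enemy is an enemy Blueprint with placeholder damage handling that destroys itself when its health is depleted.
; MoveNPC checks that Target is valid, then uses AIMoveTo with continuous goal tracking toward the player pawn rather than Target.
; The only MoveNPC call shown sits in an unconnected chain, and BeginPlay is empty.
; UpdateMoveSpeed sets the walk speed on CharacterMovement.
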(event Custom|MoveNPC
  (Utilities|IsValid (Variables|Default|GetTarget)
    (:Is%20Valid
      (AI|AIMoveTo (AI|GetAIController self) "0, 0, 0" (Game|Player|GetPlayerPawn 0) 1e+03 "Disable" "Default" true true true))))

(event EventBeginPlay)

(event EventHealthDepleted
  (Actor|DestroyActor))

(event EventDamageTaken
  (params (DamagedActor :type Actor%20Object%20Reference) (Damage :type Float%20%28single-precision%29) (DamageType :type Damage%20Type%20Object%20Reference) (InstigatedBy :type Controller%20Object%20Reference) (DamageCauser :type Actor%20Object%20Reference))
  (Development|PrintString "TODO: Enemy damaged"))

(fn ConstructionScript)

(fn UpdateMoveSpeed
  (params (NewMoveSpeed :type Float%20%28double-precision%29))
  (Variables|/Script/Engine.CharacterMovementComponent|SetMaxWalkSpeed (Variables|Character|GetCharacterMovement) NewMoveSpeed))