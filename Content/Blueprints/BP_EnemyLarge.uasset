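; BP_EnemyLarge is a large enemy character driven by an AIC_Enemy AI controller.
; On BeginPlay it passes its MaxWeaponRange to that controller as the attack range.
; When health depletes it decrements the EnemyManager's alive-enemy count and destroys itself, while the damage event only prints a TODO.
; UpdateMoveSpeed sets the character movement's max walk speed.
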(event EventBeginPlay
  ;[1 1 1] Set attack range on AI Controller
  (bind _asaic_enemy (Utilities|Casting|CastToAIC_Enemy (AI|GetAIController self)))
  (Variables|/Game/Blueprints/AIC_Enemy.AIC_Enemy_C|SetMaxWeaponRange _asaic_enemy (Variables|Default|GetMaxWeaponRange)))

(event EventHealthDepleted
  (Class|EnemyManager|DecrementNumAliveEnemies (Variables|Default|GetEnemyManager))
  (Actor|DestroyActor))

(event EventDamageTaken
  (params (DamagedActor :type Actor%20Object%20Reference) (Damage :type Float%20%28single-precision%29) (DamageType :type Damage%20Type%20Object%20Reference) (InstigatedBy :type Controller%20Object%20Reference) (DamageCauser :type Actor%20Object%20Reference))
  (Development|PrintString "TODO: Enemy damaged"))

(fn ConstructionScript)

(fn UpdateMoveSpeed
  (params (NewMoveSpeed :type Float%20%28double-precision%29))
  (Variables|/Script/Engine.CharacterMovementComponent|SetMaxWalkSpeed (Variables|Character|GetCharacterMovement) NewMoveSpeed))