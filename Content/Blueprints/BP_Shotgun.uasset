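; Shotgun weapon pickup that attaches its TPShotgun component to the character who picks it up.
; The construction script sets pellet count and hitscan range, while BeginPlay copies ammo, damage and firing settings to the component.
; BeginPlay also async-loads the fire montage, projectile class and sound, assigning each on completion.
; A leftover debug event draws random cone line traces to test spread, but its timer is disconnected.
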(event OnPickUp(TP_PickUp)
  (params (PickUpCharacter :type FPS%20Feature%20Proj%20Character%20Object%20Reference))
  (bind _tp_shotgun (Variables|Default|GetTP_Shotgun))
  (if (Utilities|IsValid _tp_shotgun)
    (Class|TPWeaponComponent|AttachWeapon _tp_shotgun PickUpCharacter)))

(event Custom|TEST_ShotgunLinecasts
  (bind _self self)
  (bind _returnvalue (Transformation|GetActorLocation _self))
  ;[0.01876 1 0] TODO: Testing: Create random shotgun vectors
  (Variables|Default|SetTEMP_ForwardVector (Transformation|GetActorForwardVector (Game|Player|GetPlayerPawn 0)))
  (for _index (range 0 100)
    (Collision|LineTraceByChannel _returnvalue (+ _returnvalue (* (Math|Random|RandomUnitVectorinConeinDegrees (Variables|Default|GetTEMP_ForwardVector) 1e+01) "500.000000,500.000000,500.000000")) "TraceTypeQuery1" false 0 "ForDuration" true "(R=1.000000,G=0.000000,B=0.000000,A=1.000000)" "(R=0.000000,G=1.000000,B=0.000000,A=1.000000)" 1e+01))
  (Development|PrintString "Created random shotgun vectors"))

(event EventBeginPlay
  (bind _tp_shotgun (Variables|Default|GetTP_Shotgun))
  ;[1 1 1] Set instance variable on BeginPlay
  (bind _output_get (Variables|/Script/FPSFeatureProj.TP_WeaponComponent|SetMaxAmmo _tp_shotgun (Variables|Default|GetMaxAmmo)))
  (Variables|/Script/FPSFeatureProj.TP_WeaponComponent|SetCurrentAmmo _tp_shotgun _output_get)
  (Variables|/Script/FPSFeatureProj.TP_WeaponComponent|SetDamage _tp_shotgun (Variables|Default|GetDamage))
  (Variables|/Script/FPSFeatureProj.TP_WeaponComponent|SetFireInterval _tp_shotgun (Variables|Default|GetFireInterval))
  (Variables|/Script/FPSFeatureProj.TP_WeaponComponent|SetIsAutomatic _tp_shotgun (Variables|Default|GetIsAutomatic))
  (Variables|/Script/FPSFeatureProj.TP_WeaponComponent|SetIsHitscan _tp_shotgun (Variables|Default|GetIsHitscan))
  (bind _object (Utilities|AsyncLoadAsset (Variables|Default|GetFireAnimation))
    (:then
      (bind _class (Utilities|AsyncLoadClassAsset (Variables|Default|GetProjectileClass))
        (:then
          (bind _object_2 (Utilities|AsyncLoadAsset (Variables|Default|GetFireSound))
            (:Completed
              (bind _assound_base (Utilities|Casting|CastToSoundBase _object_2))
              (Variables|/Script/FPSFeatureProj.TP_WeaponComponent|SetFireSound _tp_shotgun _assound_base))))
        (:Completed
          (bind _asfpsfeature_proj_projectile (Utilities|Casting|CastToFPSFeatureProjProjectileClass _class))
          (Variables|/Script/FPSFeatureProj.TP_WeaponComponent|SetProjectileClass _tp_shotgun _asfpsfeature_proj_projectile))))
    (:Completed
      (bind _asanim_montage (Utilities|Casting|CastToAnimMontage _object))
      (Variables|/Script/FPSFeatureProj.TP_WeaponComponent|SetFireAnimation _tp_shotgun _asanim_montage))))

(fn ConstructionScript
  (bind _tp_shotgun (Variables|Default|GetTP_Shotgun))
  (Variables|/Script/FPSFeatureProj.TP_ShotgunComponent|SetNumPellets _tp_shotgun (Variables|Default|GetNumPellets))
  (Variables|/Script/FPSFeatureProj.BaseWeaponComponent|SetHitscanRange _tp_shotgun (Variables|Default|GetShotgunRange)))