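; AI controller for a melee enemy that runs BT_EnemyMelee and sets player pawn 0 as its Blackboard target on possession.
; Perception of a Player-tagged actor latches HasLineOfSight, after which Tick compares distance to MaxWeaponRange and writes WithinRange only when it changes.
; StartEnemyTimer would clear sight, target and range, but its timer setup is disconnected, so nothing here triggers that reset.
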(event OnTargetPerceptionUpdated(AIPerception)
  (params (Actor :type Actor%20Object%20Reference) (Stimulus :type AI%20Stimulus%20Structure))
  (if (and (Actor|ActorHasTag Actor "Player") (.bSuccessfullySensed (Utilities|Struct|BreakAIStimulus Stimulus)))
    ;[1 1 1] If the player is seen, set Player object variable within BT_Enemy and stop wait timer.
    (Utilities|Time|ClearandInvalidateTimerbyHandle (Variables|Default|GetEnemyTimer))
    (AI|Components|Blackboard|SetValueasBool (Variables|Default|GetBlackboard) (Variables|Default|GetHasLineOfSight) true)
    (Variables|Default|SetHasLOS true)))

(event Custom|StartEnemyTimer
  (bind _blackboard (Variables|Default|GetBlackboard))
  ;[1 1 1] If player is not seen, wait some time and clear variable for Player within BT_Enemy.
  (AI|Components|Blackboard|SetValueasBool _blackboard (Variables|Default|GetHasLineOfSight) false)
  (AI|Components|Blackboard|SetValueasObject _blackboard (Variables|Default|GetEnemyActor) 0)
  (AI|Components|Blackboard|SetValueasBool _blackboard (Variables|Default|GetWithinRange) false)
  (Variables|Default|SetHasLOS false))

(event EventTick
  (params (DeltaSeconds :type Float%20%28single-precision%29))
  (bind _returnvalue (Game|Player|GetPlayerPawn 0))
  ;[1 1 1] Fire at the player if they are visible and within range.
  (if (Variables|Default|GetHasLOS)
    (Utilities|IsValid _returnvalue
      (:Is%20Valid
        (bind _output_get (Variables|Default|SetPlayerDistance (Math|Vector|Distance(Vector) (Transformation|GetActorLocation _returnvalue) (Transformation|GetActorLocation (Pawn|GetControlledPawn self))))) ; Store distance so that it only needs to be computed once per tick
        ;;[1 1 1] Only update the Blackboard value if it has changed this tick.
        (if (!= (ScalableFloat|GetValueasBool (Variables|Default|GetBlackboard) (Variables|Default|GetWithinRange)) (<= _output_get (Variables|Default|GetMaxWeaponRange)))
          (AI|Components|Blackboard|SetValueasBool (Variables|Default|GetBlackboard) (Variables|Default|GetWithinRange) (<= _output_get (Variables|Default|GetMaxWeaponRange))))))))

(event EventPossess
  (params (PossessedPawn :type Pawn%20Object%20Reference))
  (AI|RunBehaviorTree "/Game/BehaviorTrees/BT_EnemyMelee.BT_EnemyMelee")
  ;[1 1 1] Initialize Blackboard reference to Player
  (AI|Components|Blackboard|SetValueasObject (Variables|Default|GetBlackboard) (Variables|Default|GetEnemyActor) (Game|Player|GetPlayerPawn 0)))

(event EventBeginPlay)

(fn ConstructionScript)